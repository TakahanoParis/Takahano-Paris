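; Player character Blueprint for Julia, who hacks electronics she is looking at.
; Every tick it asks the CustomPlayerController for visible actors implementing InteractInterface, stores them in LookedAtElectronics and prints their names on screen.
; Each D-pad direction maps to an index in that array and calls TryHackBP on that actor, printing the result.
; The right face button blends the view target back to Julia.
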(event `self.ReceiveTick`
  (params (DeltaSeconds :type "Float (single-precision)"))
  (`self.SetArrayLookedAtElectronics`))

(event `Key|AnyKey`
  (params (Key :type "Key Structure"))
  (bind _lookedatelectronics (`self.LookedAtElectronics`))
  (bind _returnvalue (`KismetArrayLibrary.Array_Find` (`|MakeArray` "Gamepad_DPad_Up" "Gamepad_DPad_Right" "Gamepad_DPad_Down" "Gamepad_DPad_Left" :!type "Key Structure") Key))
  (:`Pressed`
    (if (`KismetArrayLibrary.Array_IsValidIndex` _lookedatelectronics _returnvalue)
      (bind _returnvalue_2 (`self.TryHack_BP` (`|GetArrayItem` _lookedatelectronics _returnvalue)))
      (`KismetSystemLibrary.PrintString` (`KismetStringLibrary.Conv_BoolToString` _returnvalue_2)))))

(event `Key|Gamepad_FaceButton_Right`
  (params (Key :type "Key Structure"))
  (:`Pressed`
    (bind _asplayer_controller (cast `PlayerController` (`self.GetController`)))
    (`PlayerController.SetViewTargetWithBlend` _asplayer_controller self 0.1 "VTBlend_EaseInOut" 0.0 false)))

(fn `SetArrayLookedAtElectronics`
  (bind _ascustom_player_controller (cast `CustomPlayerController` (`self.GetController`)))
  (bind _output_get (set `self.LookedAtElectronics` (`CustomPlayerController.GetVisibleActorsWithInterface_BP` _ascustom_player_controller "/Script/TakahanoParis.InteractInterface")))
  (for _array_element _output_get
    (`KismetSystemLibrary.PrintString` (`KismetSystemLibrary.GetDisplayName` _array_element) true false (struct :`G` 0.66 :`B` 1.0 :`A` 1.0) 0.0)))

(fn `UserConstructionScript`)