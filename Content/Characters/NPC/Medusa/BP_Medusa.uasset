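; BP_Medusa is an NPC character Blueprint for Medusa that deals heavy contact damage to actors of another team.
; When AttackSphere begins overlapping an actor, it compares both teams through a team getter interface and applies a large hit if they differ, crediting its controller as instigator.
; Tick prints the custom character movement component's SpeedDelta to the screen each frame as debug output.
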(event `self.ReceiveTick`
  (params (DeltaSeconds :type "Float (single-precision)"))
  (bind _ascustom_character_movement_component (cast `CustomCharacterMovementComponent` (`self.CharacterMovement`)))
  (`KismetSystemLibrary.PrintString` (`KismetStringLibrary.Conv_DoubleToString` (`CustomCharacterMovementComponent.SpeedDelta` _ascustom_character_movement_component)) true true (struct :`G` 0.66 :`B` 1.0 :`A` 1.0) 0.0))

(event `self.AttackSphere.OnComponentBeginOverlap`
  (params (OverlappedComponent :type "PrimitiveComponent Object Reference") (OtherActor :type "Actor Object Reference") (OtherComp :type "PrimitiveComponent Object Reference") (OtherBodyIndex :type Integer) (bFromSweep :type Boolean) (SweepResult :type "HitResult Structure (by ref)"))
  (bind _returnvalue (`TeamInterface.I_GetTeam_BP` self))
  (bind _returnvalue_2 (message `TeamInterface.I_GetTeam_BP` OtherActor))
  (if (!= _returnvalue_2 _returnvalue)
    (`GameplayStatics.ApplyDamage` OtherActor 1000.0 (`self.GetController`) self "/Script/Engine.DamageType")))

(fn `UserConstructionScript`)